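; Board actor that procedurally builds an irregular, index-labelled tile map at construction and spawns BP_Char on the last tile placed at BeginPlay.
; The construction script lays a square grid of arrow components as position anchors, then places a central mesh tile.
; It grows the map to roughly three quarters of the grid by repeatedly picking a random used cell's neighbour, retrying until the index is in range and unused.
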(event EventBeginPlay
  (bind _used_indexes (Variables|Memory|GetUsed_Indexes))
  (Utilities|FlowControl|Sequence
    (:then_1
      (Game|SpawnActorfromClass "/Game/BP/BP_Char.BP_Char_C" (Math|Conversions|ToTransform(Vector) (Transformation|GetWorldLocation (Utilities|Array|Get(acopy) (Variables|Memory|GetAll_Arrows) (Utilities|Array|Get(acopy) _used_indexes (Utilities|Array|LastIndex _used_indexes))))) "Undefined" 0 0))))

(fn ConstructionScript
  (Utilities|FlowControl|Sequence
    (:then_0
      (Variables|BoardSize|SetX_Quantity (Math|Float|Truncate (Math|Float|Sqrt (Math|Conversions|ToFloat(Integer) (Variables|BoardSize|GetHowManyArrows)))))
      (Variables|BoardSize|SetY_Quantity (Math|Float|Truncate (Math|Float|Sqrt (Math|Conversions|ToFloat(Integer) (Variables|BoardSize|GetHowManyArrows)))))
      (for _index (range 0 (- (Variables|BoardSize|GetHowManyArrows) 1))
        (bind _returnvalue (AddComponent|AddArrowComponent false (Math|Transform|MakeTransform (Math|Conversions|ToVector(Float) (Utilities|Struct|MakeIntVector (* (/ _index (Variables|BoardSize|GetX_Quantity)) (Variables|BoardSize|GetSize)) (* (Math|Integer|%(Integer) _index (Variables|BoardSize|GetY_Quantity)) (Variables|BoardSize|GetSize)))) "90.000000,0.000000,0.000000" "1.000000,1.000000,1.000000")))
        (Utilities|Array|Add (Variables|Memory|GetAll_Arrows) _returnvalue)))
    (:then_1
      (bind _output_get (Variables|Memory|SetCentral_Arrow (- (/ (Variables|BoardSize|GetHowManyArrows) 2) (/ (Variables|BoardSize|GetX_Quantity) 2)))) ; Get Centeral Arrow Index
      (Utilities|Array|Add (Variables|Memory|GetUsed_Indexes) _output_get)
      (AddComponent|AddStaticMeshComponent false (Math|Transform|MakeTransform (Math|Vector|MakeVector (.x (Transformation|GetWorldLocation (Utilities|Array|Get(acopy) (Variables|Memory|GetAll_Arrows) _output_get))) (.y (Transformation|GetWorldLocation (Utilities|Array|Get(acopy) (Variables|Memory|GetAll_Arrows) _output_get))) 0.0) "0, 0, 0" "0.900000,0.900000,0.900000"))
      (Utilities|FlowControl|ForLoopwithBreak 0 (Math|ThreeFourthOfArrowsAmount)
        (:LoopBody
          (bind _out (Construction|CheckValidIndex))
          (LocalVariables|SetLocal_Get_Index _out)
          (AddComponent|AddStaticMeshComponent false (Math|Transform|MakeTransform (Math|Vector|MakeVector (.x (Transformation|GetWorldLocation (Utilities|Array|Get(acopy) (Variables|Memory|GetAll_Arrows) (LocalVariables|GetLocal_Get_Index)))) (.y (Transformation|GetWorldLocation (Utilities|Array|Get(acopy) (Variables|Memory|GetAll_Arrows) (LocalVariables|GetLocal_Get_Index)))) 0.0) "0, 0, 0" "0.900000,0.900000,0.900000"))
          (bind _returnvalue_2 (AddComponent|AddTextRenderComponent false (Math|Transform|MakeTransform (Math|Vector|MakeVector (.x (Transformation|GetWorldLocation (Utilities|Array|Get(acopy) (Variables|Memory|GetAll_Arrows) (LocalVariables|GetLocal_Get_Index)))) (.y (Transformation|GetWorldLocation (Utilities|Array|Get(acopy) (Variables|Memory|GetAll_Arrows) (LocalVariables|GetLocal_Get_Index)))) 2.0) "90.000000,180.000000, 0" "1.000000,1.000000,1.000000")))
          (Rendering|Components|TextRender|SetText _returnvalue_2 (Utilities|Text|ToText(Integer) (LocalVariables|GetLocal_Get_Index)))
          (Utilities|Array|Add (Variables|Memory|GetUsed_Indexes) (LocalVariables|GetLocal_Get_Index)))))))

(fn SetSquareRef
  (Utilities|IsValid (Variables|Ref|GetSquare_Ref)
    (:Is%20Not%20Valid
      (bind _returnvalue (Actor|GetActorOfClass "/Game/BP/BP_Square.BP_Square_C"))
      (Variables|Ref|SetSquare_Ref _returnvalue))))

(fn ThreeFourthOfArrowsAmount
  (return (- (Variables|BoardSize|GetHowManyArrows) (/ (Variables|BoardSize|GetHowManyArrows) 4))))

(fn IndexAround
  (LocalVariables|SetLoc_Int (.OutItem (Utilities|Array|Random (Variables|Memory|GetUsed_Indexes))))
  (switch int (Math|Random|RandomInteger 4)
    (:0
      (return (- (LocalVariables|GetLoc_Int) (Variables|BoardSize|GetX_Quantity))))
    (:1
      (return (- (LocalVariables|GetLoc_Int) 1)))
    (:2
      (return (+ (LocalVariables|GetLoc_Int) (Variables|BoardSize|GetX_Quantity))))
    (:3
      (return (+ (LocalVariables|GetLoc_Int) 1)))))

(fn CheckValidIndex
  (bind _index (Construction|IndexAround :!label _label))
  (if (and (> _index 0) (< _index (Variables|BoardSize|GetHowManyArrows)))
    (LocalVariables|SetLocal_Int _index)
    (bind _array_element (Utilities|Array|ForEachLoopwithBreak (Variables|Memory|GetUsed_Indexes))
      (:LoopBody
        (if (not (!= (LocalVariables|GetLocal_Int) _array_element))
          (goto _label)))
      (:Completed
        (return (LocalVariables|GetLocal_Int))))
    (else
      (goto _label))))