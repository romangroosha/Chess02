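; BP_Camera is a camera actor that appears meant to follow BP_Char, but its movement logic is currently disconnected.
; BeginPlay and the Down_Left_Up_Right direction event are empty.
; Unwired nodes would cache the player controller, character and board, snap to the character after a delay, and register for directional input.
; An unwired 0To1 timeline would lerp the actor toward the character's location.
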(event Custom|Down_Left_Up_Right
  (params (Direction :type Integer)))

(event EventBeginPlay)

(fn ConstructionScript)

(fn SetBoardRef
  (Utilities|IsValid (Variables|Default|GetBoard_Ref)
    (:Is%20Not%20Valid
      (bind _returnvalue (Actor|GetActorOfClass "/Game/BP/BP_Board.BP_Board_C"))
      (Variables|Default|SetBoard_Ref _returnvalue))))

(fn SetCharRef
  (Utilities|IsValid (Variables|Default|GetChar_Ref)
    (:Is%20Not%20Valid
      (bind _returnvalue (Actor|GetActorOfClass "/Game/BP/BP_Char.BP_Char_C"))
      (Variables|Default|SetChar_Ref _returnvalue))))

(fn SetPlayerControllerRef
  (Utilities|IsValid (Variables|Default|GetPlayerController_Ref)
    (:Is%20Not%20Valid
      (bind _asbp_player_controller (Utilities|Casting|CastToBP_PlayerController (Game|GetPlayerController 0)))
      (Variables|Default|SetPlayerController_Ref _asbp_player_controller))))