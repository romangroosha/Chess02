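; BP_Char is a character that moves one cell at a time across the BP_Board grid and serves as the player's view target.
; BP_PlayerController supplies a direction (down, left, up, right) to its bound event.
; The current cell is found by matching arrow world locations, then neighbour indices derive from the board width and are checked against used indexes.
; A timeline lerps to the target arrow, with a flag blocking input meanwhile.
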(event Custom|Down_Left_Up_Right_Event
  (params (Direction :type Integer))
  (if (Variables|Move|GetIsMoveAnimationFinished)
    (Variables|Move|SetIsMoveAnimationFinished false)
    ;[1 1 1] Move BP_Char. Checks if BP_Char is moving on used index
    (bind _index (Move|GetActorCurrentIndex))
    (bind _index_2 (Move|FourIndexAround _index))
    (Variables|Move|SetFour_Index _index_2)
    (bind _out (Move|CheckValidIndex (Utilities|Array|Get(acopy) _index_2 Direction)))
    (Variables|Default|SetArrowLocationByIndex (Transformation|GetWorldLocation (Utilities|Array|Get(acopy) (Variables|/Game/BP/BP_Board.BP_Board_C|GetAll_Arrows (Variables|Ref|GetBoard_Ref)) (Utilities|Array|Get(acopy) _index_2 Direction))))
    (Variables|Default|SetCurrentActorLocation (Transformation|GetActorLocation))
    (if (== _out -1)
      (Development|PrintString)
      (else
        (bind _0_to_1_track (Timeline|Timeline_0 PlayFromStart)
          (:Update
            (Transformation|SetActorLocation (Math|Vector|Lerp(Vector) (Variables|Default|GetCurrentActorLocation) (Variables|Default|GetArrowLocationByIndex) _0_to_1_track) false false))
          (:Finished
            (Variables|Move|SetIsMoveAnimationFinished true)))))
    (else
      (Development|PrintString "Hello"))))

(event EventBeginPlay
  (Ref|SetCameraRef)
  (Ref|SetBoardRef)
  (Ref|SetPlayerControllerRef)
  (EventDispatchers|AssignDownLeftUpRight (Variables|Ref|GetPlayerController_Ref) (EventDispatchers|CreateEvent :!event Custom|Down_Left_Up_Right_Event)) ; Assign event for moving
  (Game|Player|SetViewTargetwithBlend (Variables|Ref|GetPlayerController_Ref) self 0.0 "VTBlend_Linear" 0.0 false) ; Bind Camera to BP_Char
)

(fn ConstructionScript)

(fn SetPlayerControllerRef
  (Utilities|IsValid (Variables|Ref|GetPlayerController_Ref)
    (:Is%20Not%20Valid
      (bind _asbp_player_controller (Utilities|Casting|CastToBP_PlayerController (Game|GetPlayerController 0)))
      (Variables|Ref|SetPlayerController_Ref _asbp_player_controller))))

(fn SetBoardRef
  (Utilities|IsValid (Variables|Ref|GetBoard_Ref)
    (:Is%20Not%20Valid
      (bind _returnvalue (Actor|GetActorOfClass "/Game/BP/BP_Board.BP_Board_C"))
      (Variables|Ref|SetBoard_Ref _returnvalue))))

(fn CheckValidIndex
  (params (In :type Integer))
  (LocalVariables|SetLoc_Int In)
  (bind _array_element (Utilities|Array|ForEachLoopwithBreak (Variables|/Game/BP/BP_Board.BP_Board_C|GetUsed_Indexes_Arrows (Variables|Ref|GetBoard_Ref)) :!label _label)
    (:LoopBody
      (if (== _array_element (LocalVariables|GetLoc_Int))
        (LocalVariables|SetNot_Contain false)
        (goto _label Break)
        (else
          (LocalVariables|SetNot_Contain true))))
    (:Completed
      (if (LocalVariables|GetNot_Contain)
        (return -1)
        (else
          (return (LocalVariables|GetLoc_Int)))))))

(fn FourIndexAround
  (params (In :type Integer))
  (LocalVariables|SetLoc_Int In)
  (if (== (Math|Integer|%(Integer) (LocalVariables|GetLoc_Int) (Variables|/Game/BP/BP_Board.BP_Board_C|GetX_Quantity (Variables|Ref|GetBoard_Ref))) 0)
    (LocalVariables|SetLoc_Left (LocalVariables|GetLoc_Int))
    (else
      (LocalVariables|SetLoc_Left (- (LocalVariables|GetLoc_Int) 1))))
  (if (== (Math|Integer|%(Integer) (+ (LocalVariables|GetLoc_Int) 1) (Variables|/Game/BP/BP_Board.BP_Board_C|GetX_Quantity (Variables|Ref|GetBoard_Ref))) 0)
    (LocalVariables|SetLoc_Right (LocalVariables|GetLoc_Int))
    (else
      (LocalVariables|SetLoc_Right (+ (LocalVariables|GetLoc_Int) 1))))
  (return (Utilities|Array|MakeArray (- (LocalVariables|GetLoc_Int) (Variables|/Game/BP/BP_Board.BP_Board_C|GetX_Quantity (Variables|Ref|GetBoard_Ref))) (LocalVariables|GetLoc_Left) (+ (LocalVariables|GetLoc_Int) (Variables|/Game/BP/BP_Board.BP_Board_C|GetX_Quantity (Variables|Ref|GetBoard_Ref))) (LocalVariables|GetLoc_Right))))

(fn GetActorCurrentIndex
  (bind _array_element (Utilities|Array|ForEachLoopwithBreak (Variables|/Game/BP/BP_Board.BP_Board_C|GetUsed_Indexes_Arrows (Variables|Ref|GetBoard_Ref)) :!label _label)
    (:LoopBody
      (if (Utilities|Operators|EqualEqual (Transformation|GetWorldLocation (Utilities|Array|Get(acopy) (Variables|/Game/BP/BP_Board.BP_Board_C|GetAll_Arrows (Variables|Ref|GetBoard_Ref)) _array_element)) (Transformation|GetActorLocation) 0.0)
        (goto _label Break)))
    (:Completed
      (return _array_element))))

(fn SetCameraRef
  (Utilities|IsValid (Variables|Ref|GetCamera_Ref)
    (:Is%20Not%20Valid
      (bind _returnvalue (Actor|GetActorOfClass "/Game/BP/BP_Camera.BP_Camera_C"))
      (Variables|Ref|SetCamera_Ref _returnvalue))))