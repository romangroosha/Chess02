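; BP_Square is a board piece that, on BeginPlay, extends a capped chain of spawns on BP_Board's arrow grid.
; While the board's SquareCounter is within about three quarters of HowManySquares, it increments the counter and spawns an actor beside CentralArrow.
; IndexAround picks the neighbor by offsetting the flat grid index by one or XQuantity.
; RandomInteger(3) yields only 0–2, so the "right" case is never chosen.
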(event EventBeginPlay
  (CallFunction|SetBoardRef)
  (if (CallFunction|ThreeFourthOfArrowsAmount)
    (Math|Integer|IncrementInt (Variables|/Game/BP/BP_Board.BP_Board_C|GetSquare_Counter (Variables|Ref|GetBoard_Ref))
      (:%20%20
        (bind _index (CallFunction|IndexAround))
        (Game|SpawnActorfromClass "BP_Square_C" (Math|Conversions|ToTransform(Vector) (Transformation|GetWorldLocation (Utilities|Array|Get(acopy) (Variables|/Game/BP/BP_Board.BP_Board_C|GetAll_Arrows (Variables|Ref|GetBoard_Ref)) _index))) "Undefined" 0 0)))))

(fn ConstructionScript)

(fn SetBoardRef
  (Utilities|IsValid (Variables|Ref|GetBoard_Ref)
    (:Is%20Not%20Valid
      (bind _returnvalue (Actor|GetActorOfClass "/Game/BP/BP_Board.BP_Board_C"))
      (Variables|Ref|SetBoard_Ref _returnvalue))))

(fn IndexAround
  (bind _board_ref (Variables|Ref|GetBoard_Ref))
  (bind _board_ref_2 (Variables|Ref|GetBoard_Ref))
  (switch int (Math|Random|RandomInteger 3)
    (:0
      (return (- (Variables|/Game/BP/BP_Board.BP_Board_C|GetCentral_Arrow _board_ref_2) (Variables|/Game/BP/BP_Board.BP_Board_C|GetX_Quantity _board_ref_2))))
    (:1
      (return (- (Variables|/Game/BP/BP_Board.BP_Board_C|GetCentral_Arrow (Variables|Ref|GetBoard_Ref)) 1)))
    (:2
      (return (+ (Variables|/Game/BP/BP_Board.BP_Board_C|GetCentral_Arrow _board_ref) (Variables|/Game/BP/BP_Board.BP_Board_C|GetX_Quantity _board_ref))))
    (:3
      (return (+ (Variables|/Game/BP/BP_Board.BP_Board_C|GetCentral_Arrow (Variables|Ref|GetBoard_Ref)) 1)))))

(fn ThreeFourthOfArrowsAmount
  (bind _board_ref (Variables|Ref|GetBoard_Ref))
  (return (<= (Variables|/Game/BP/BP_Board.BP_Board_C|GetSquare_Counter _board_ref) (- (Variables|/Game/BP/BP_Board.BP_Board_C|GetHowManySquares _board_ref) (/ (Variables|/Game/BP/BP_Board.BP_Board_C|GetHowManySquares _board_ref) 4)))))